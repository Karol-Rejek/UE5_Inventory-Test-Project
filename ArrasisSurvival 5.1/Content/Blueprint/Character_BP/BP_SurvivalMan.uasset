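; BP_SurvivalMan is a character Blueprint whose only logic is an inventory UI toggle, currently not wired to any event.
; The unconnected FlipFlop alternates between creating an InventoryBase widget with Game and UI input and a visible cursor, and removing it to restore game-only input.
; BeginPlay and the construction script are empty, so the toggle never runs.
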(event EventBeginPlay)

(event Input|KeyboardEvents|I
  (params (Key :type Key%20Structure :default "None")))

(fn ConstructionScript)