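; BP_SurvivalMan is a character Blueprint that handles opening and closing the inventory screen.
; The I key drives a FlipFlop that creates a new InventoryBase widget on one press and removes it from the viewport on the next.
; Opening shows the mouse cursor with Game and UI input mode, and closing restores game-only input and hides the cursor.
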(event EventBeginPlay)

(event Input|KeyboardEvents|I
  (params (Key :type Key%20Structure :default "None"))
  (bind _returnvalue (Game|GetPlayerController 0))
  (:Pressed
    (Utilities|FlowControl|FlipFlop
      (:A
        (bind _returnvalue_2 (UserInterface|CreateWidget "/Game/Widgets/character/InventoryWidgets/InventoryBase.InventoryBase_C"))
        (bind _output_get (Variables|Default|SetInventoryUIReference _returnvalue_2))
        (UserInterface|Viewport|AddtoViewport _output_get 0)
        (Input|SetInputModeGameandUI _returnvalue 0 "DoNotLock" false)
        (Variables|/Script/Engine.PlayerController|SetbShowMouseCursor _returnvalue true))
      (:B
        (if (Utilities|IsValid (Variables|Default|GetInventoryUIReference))
          (Widget|RemovefromParent (Variables|Default|GetInventoryUIReference))
          (Input|SetInputModeGameOnly _returnvalue)
          (Variables|/Script/Engine.PlayerController|SetbShowMouseCursor _returnvalue false))))))

(fn ConstructionScript)